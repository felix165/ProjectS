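; BP_Arena runs a timed battle between two agent teams, serving both chromosome-based training and regular matches.
; Training randomly spawns both teams with Manager-assigned chromosomes; matches build Team A preparation tiles and spawn Team B with GameInstance chromosomes.
; Battles spawn buff items on a timer, and Tick resolves win or tie, reporting to Manager or HUD.
; GetBattleInformation exposes per-team damage, survivor, kill, HP and time stats.
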(event `self.ReceiveBeginPlay`
  (set `self.TeamA_Damage` 0.0)
  (set `self.TeamB_Damage` 0.0)
  (set `self.MaxHpA` 0.0)
  (set `self.MaxHpB` 0.0)
  (if (not (`self.isTraining?`))
    (`self.SpawnTileA`)
    (set `self.TeamSize` (`/Game/Blueprints/GI_Main.Agent Amount` (`self.Get_GI`)))
    (`self.PreparationMode`)
    (`SceneComponent.SetVisibility` (`self.TrainingInfo`) false true)))

(event `self.ReceiveTick`
  (params (DeltaSeconds :type "Float (single-precision)"))
  (bind _hud (`self.GetHUD`))
  (bind _curtime (`self.CurTime`))
  (bind _battlestate (`self.BattleState`))
  (`TextRenderComponent.K2_SetText` (`self.State`) (`KismetTextLibrary.Conv_StringToText` (`KismetStringLibrary.Concat_StrStr` "Arena - " (`KismetStringLibrary.Conv_IntToString` (`self.IndexArena`)) " \n" (`|GetEnumeratorNameAsString` _battlestate))))
  (`TextRenderComponent.K2_SetText` (`self.Time`) (`KismetTextLibrary.Conv_StringToText` (`KismetStringLibrary.Concat_StrStr` (`KismetStringLibrary.Conv_IntToString` (/ (`KismetMathLibrary.FTrunc` _curtime) 60)) " : " (`KismetStringLibrary.Conv_IntToString` (mod (`KismetMathLibrary.FTrunc` _curtime) 60)))))
  (switch `/Game/Blueprints/Property/E_BattleState` _battlestate
    (:`NewEnumerator1`
      (bind _output_get (set `self.CurTime` (- (`self.CurTime`) (`GameplayStatics.GetWorldDeltaSeconds`))))
      (if (<= _output_get 0.0)
        (set `self.BattleState` "NewEnumerator4")
        (`self.CheckBattleState`)
        (else
          (`self.CheckBattleState`))))
    (:`NewEnumerator2`
      (`/Engine/EditorBlueprintResources/StandardMacros.DoOnce` false :!label _label
        (:`Completed`
          (if (`self.isTraining?`)
            (`/Game/Blueprints/Property/BP_TrainingManager.FightFinished` (`self.Manager`) self _battlestate)
            (else
              (switch `/Game/Blueprints/Property/E_BattleState` _battlestate
                (:`NewEnumerator2`
                  (`/Game/Blueprints/HUD_Main.BattleEnd` _hud true))
                (:`NewEnumerator3`
                  (`/Game/Blueprints/HUD_Main.BattleEnd` _hud false)))))
          (`KismetSystemLibrary.K2_ClearAndInvalidateTimerHandle` (`self.SpawnItemHandle`)))))
    (:`NewEnumerator3`
      (goto _label))
    (:`NewEnumerator4`
      (goto _label))))

(event `Start Training`
  (`self.PreparationMode`)
  (`KismetSystemLibrary.Delay` 1.0)
  (`self.SpawnAgent4Training` true)
  (`self.SpawnAgent4Training` false)
  (`self.Start Battle`))

(event `Start Battle`
  (`self.Set Preparation Component Visibility` false)
  (`self.ActivateAgent`)
  (set `self.BattleState` "NewEnumerator1")
  (`KismetSystemLibrary.Delay` 2.0)
  (bind _returnvalue (`KismetSystemLibrary.K2_SetTimer` null "SpawnItemsBuff" 20.0 true -2.0))
  (set `self.SpawnItemHandle` _returnvalue))

(event `Set Preparation Component Visibility`
  (params (bNewVisibility :type Boolean))
  (`SceneComponent.SetVisibility` (`self.Preparation`) bNewVisibility true))

(event `PreparationMode`
  (`self.Set Preparation Component Visibility` true)
  (set `self.CurTime` (`self.TotalTime`))
  (set `self.BattleState` "NewEnumerator0")
  (if (not (`self.isTraining?`))
    (`self.SpawnAgent4Battle` false)))

(event `Reset_Event`
  (bind _teamsb (`self.TeamsB`))
  (bind _teamsa (`self.TeamsA`))
  (for _array_element _teamsa
    (`/Engine/EditorBlueprintResources/StandardMacros.IsValid` _array_element
      (:`Is Valid`
        (`/Game/Blueprints/Characters/BP_BaseAgent.Remove Agent` _array_element))))
  (`KismetArrayLibrary.Array_Clear` _teamsa)
  (for _array_element_2 _teamsb
    (`/Engine/EditorBlueprintResources/StandardMacros.IsValid` _array_element_2
      (:`Is Valid`
        (`/Game/Blueprints/Characters/BP_BaseAgent.Remove Agent` _array_element_2))))
  (`KismetArrayLibrary.Array_Clear` _teamsb)
  (`self.SpawnAgent4Battle` false))

(fn `ActivateAgent`
  (for _array_element (`self.TeamsA`)
    (`/Game/Blueprints/Characters/BP_BaseAgent.Event Start Battle` _array_element))
  (for _array_element_2 (`self.TeamsB`)
    (`/Game/Blueprints/Characters/BP_BaseAgent.Event Start Battle` _array_element_2))
  (return))

(fn `CheckBattleState`
  (locals (FlagA :type Boolean) (FlagB :type Boolean))
  (set `local.FlagA` false)
  (set `local.FlagB` false)
  (for _array_element (`self.TeamsA`)
    (`/Engine/EditorBlueprintResources/StandardMacros.IsValid` _array_element
      (:`Is Valid`
        (switch `/Game/Blueprints/Characters/E_State` (`/Game/Blueprints/Characters/BP_BaseAgent.State` _array_element)
          (:`NewEnumerator2`
            (set `local.FlagA` true)
            (break))))))
  (for _array_element_2 (`self.TeamsB`)
    (`/Engine/EditorBlueprintResources/StandardMacros.IsValid` _array_element_2
      (:`Is Valid`
        (switch `/Game/Blueprints/Characters/E_State` (`/Game/Blueprints/Characters/BP_BaseAgent.State` _array_element_2)
          (:`NewEnumerator2`
            (set `local.FlagB` true)
            (break))))))
  (if (and (`local.FlagB`) (`local.FlagA`) (<= (`self.CurTime`) 0.0))
    (set `self.BattleState` "NewEnumerator4")
    (return)
    (elif (`local.FlagA`)
      (if (`local.FlagB`)
        (return)
        (else
          (set `self.BattleState` "NewEnumerator2")
          (return)))
      (else
        (set `self.BattleState` "NewEnumerator3")
        (return)))))

(fn `Get_GI`
  (returns (GI :type "/Game/Blueprints/GI_Main Object Reference"))
  (`self.GI`
    (:`then`
      _)
    (:`else`
      (bind _asgi_main (cast `/Game/Blueprints/GI_Main` (`GameplayStatics.GetGameInstance`))
        (:`then`
          (set `self.GI` _asgi_main))
        (:`CastFailed`
          _))))
  (return (`self.GI`)))

(fn `GetBattleInformation`
  (params (isTeamA :type Boolean))
  (returns (DamageDealt :type "Float (double-precision)") (`Jumlah Hidup` :type "Float (double-precision)") (`Jumlah Enemy Mati` :type "Float (double-precision)") (`Total Hp` :type "Float (double-precision)") (`Time Left` :type "Float (double-precision)") (`Total Damage` :type "Float (double-precision)") (`Team Size` :type "Float (double-precision)") (`Total Max Hp` :type "Float (double-precision)") (`Max Time` :type "Float (double-precision)"))
  (locals (TotalAgentA :type "Float (double-precision)") (TotalAgentB :type "Float (double-precision)") (TotalHP_A :type "Float (double-precision)" :default 0.0) (TotalHP_B :type "Float (double-precision)" :default 0.0) (TotalMaxHp_A :type "Float (double-precision)" :default 0.0) (TotalMaxHp_B :type "Float (double-precision)" :default 0.0))
  ;[1 1 1] Clear Value
  (set `local.TotalAgentA` 0.0)
  (set `local.TotalAgentB` 0.0)
  (set `local.TotalHP_A` 0.0)
  (set `local.TotalHP_B` 0.0)
  (for _array_element (`self.TeamsA`)
    (`/Engine/EditorBlueprintResources/StandardMacros.IsValid` _array_element
      (:`Is Valid`
        (if (`|EnumInequality` (`/Game/Blueprints/Characters/BP_BaseAgent.State` _array_element) "NewEnumerator4")
          (`/Engine/EditorBlueprintResources/StandardMacros.IncrementFloat` (`local.TotalAgentA`)
            (:`  `
              (set `local.TotalHP_A` (+ (`local.TotalHP_A`) (`/Game/Blueprints/Characters/BP_BaseAgent.CurHP` _array_element)))))))))
  (for _array_element_2 (`self.TeamsB`)
    (`/Engine/EditorBlueprintResources/StandardMacros.IsValid` _array_element_2
      (:`Is Valid`
        (if (`|EnumInequality` (`/Game/Blueprints/Characters/BP_BaseAgent.State` _array_element_2) "NewEnumerator4")
          (`/Engine/EditorBlueprintResources/StandardMacros.IncrementFloat` (`local.TotalAgentB`)
            (:`  `
              (set `local.TotalHP_B` (+ (`local.TotalHP_B`) (`/Game/Blueprints/Characters/BP_BaseAgent.CurHP` _array_element_2)))))))))
  (if isTeamA
    (return (`self.TeamA_Damage`) (`local.TotalAgentA`) (- (`self.TeamSize`) (`local.TotalAgentB`)) (`local.TotalHP_A`) (`self.CurTime`) (+ (`self.TeamA_Damage`) (`self.TeamB_Damage`)) (`KismetMathLibrary.Conv_IntToDouble` (`self.TeamSize`)) (`self.MaxHpA`) (`self.TotalTime`))
    (else
      (return (`self.TeamB_Damage`) (`local.TotalAgentB`) (- (`self.TeamSize`) (`local.TotalAgentA`)) (`local.TotalHP_B`) (`self.CurTime`) (+ (`self.TeamA_Damage`) (`self.TeamB_Damage`)) (`KismetMathLibrary.Conv_IntToDouble` (`self.TeamSize`)) (`self.MaxHpB`) (`self.TotalTime`)))))

(fn `GetHUD`
  (returns (HUD :type "/Game/Blueprints/HUD_Main Object Reference"))
  (`self.HUD`
    (:`then`
      _)
    (:`else`
      (bind _ashud_main (cast `/Game/Blueprints/HUD_Main` (`PlayerController.GetHUD` (`GameplayStatics.GetPlayerController` 0)))
        (:`then`
          (set `self.HUD` _ashud_main))
        (:`CastFailed`
          _))))
  (return (`self.HUD`)))

(fn `GetTileIndexFromLoc`
  (params (Value :type "Vector2D Structure"))
  (returns (X_Index :type Integer) (Y_Index :type Integer) (IsValid :type Boolean))
  (locals (x :type Integer) (y :type Integer))
  (bind (_teamatileareah_min _teamatileareah_max) (break `/Game/Blueprints/Property/S_Range` (`self.TeamATileAreaH`)))
  (bind _tilesize (`self.TileSize`))
  (bind _tilesize_2 (`self.TileSize`))
  (bind _returnvalue (* _tilesize -1.0))
  (set `local.x` (`KismetMathLibrary.FTrunc` (/ (+ Value_X (select `bool` (< Value_X 0.0) :`false` _tilesize :`true` _returnvalue)) _tilesize_2)))
  (set `local.y` (`KismetMathLibrary.FTrunc` (/ (+ Value_Y (select `bool` (< Value_Y 0.0) :`false` _tilesize :`true` _returnvalue)) _tilesize_2)))
  (return (`local.x`) (`local.y`) (`KismetMathLibrary.InRange_IntInt` (`local.x`) _teamatileareah_max _teamatileareah_min)))

(fn `GetValueFromTileIndex`
  (params (Index :type Integer))
  (returns (ReturnValue :type "Float (double-precision)"))
  (bind _tilesize (`self.TileSize`))
  (return (- (* Index _tilesize) (/ _tilesize (`KismetMathLibrary.SelectFloat` 2.0 -2.0 (> Index 0))))))

(fn `On Battle End`
  (`KismetSystemLibrary.K2_ClearAndInvalidateTimerHandle` (`self.SpawnItemHandle`))
  (for _array_element (`self.Items Buff`)
    (`/Engine/EditorBlueprintResources/StandardMacros.IsValid` _array_element
      (:`Is Valid`
        (`self.K2_DestroyActor` _array_element))))
  (for _array_element_2 (`self.TeamsA`)
    (`/Engine/EditorBlueprintResources/StandardMacros.IsValid` _array_element_2
      (:`Is Valid`
        (`/Game/Blueprints/Characters/BP_BaseAgent.Remove Agent` _array_element_2))))
  (for _array_element_3 (`self.TeamsB`)
    (`/Engine/EditorBlueprintResources/StandardMacros.IsValid` _array_element_3
      (:`Is Valid`
        (`/Game/Blueprints/Characters/BP_BaseAgent.Remove Agent` _array_element_3))))
  (for _array_element_4 (`self.Tiles`)
    (`/Engine/EditorBlueprintResources/StandardMacros.IsValid` _array_element_4
      (:`Is Valid`
        (`self.K2_DestroyActor` _array_element_4))))
  (`self.K2_DestroyActor`)
  (return))

(fn `SpawnAgent4Battle`
  (params (`isTeamA?` :type Boolean))
  (locals (Agent :type "/Game/Blueprints/Characters/BP_BaseAgent Object Reference") (Temp :type "Array of Vector2D Structure") (X :type Integer) (Y :type Integer :default 0) (`Agent Class Enum` :type "/Game/Blueprints/Characters/E_AgentClass Enum"))
  (bind _gi (`self.Get_GI`))
  (bind _agent (`local.Agent`))
  (bind (_tileareav_min _tileareav_max) (break `/Game/Blueprints/Property/S_Range` (`self.TileAreaV`)))
  (bind _returnvalue (`SceneComponent.K2_GetComponentToWorld` (`self.DefaultSceneRoot`)))
  (bind _maxhp (`/Game/Blueprints/Characters/BP_BaseAgent.MaxHp` _agent))
  (bind _value (`BlueprintMapLibrary.Map_Find` (`self.TileAreaHForAgent`) (select `/Game/Blueprints/Characters/E_AgentClass` (`local.Agent Class Enum`) :`NewEnumerator0` "/Game/Blueprints/Characters/BP_Swordsman.BP_Swordsman_C" :`NewEnumerator1` "/Game/Blueprints/Characters/BP_Shooter.BP_Shooter_C" :`NewEnumerator2` "/Game/Blueprints/Characters/BP_StaffFighter.BP_StaffFighter_C" :!type "/Game/Blueprints/Characters/BP_BaseAgent Class Reference")))
  (bind _returnvalue_2 (`KismetMathLibrary.RandomIntegerInRange` (break `/Game/Blueprints/Property/S_Range` _value) (`.Max_12_950AF26D437BFC0371E1F1A81C10CB70` (break `/Game/Blueprints/Property/S_Range` _value))))
  (`KismetArrayLibrary.Array_Clear` (`local.Temp`))
  (for _ (range 1 (+ (`self.TeamSize`) 1))
    (set `local.Agent Class Enum` (`KismetArrayLibrary.Array_Random` (`self.Agent Class`)))
    (set `local.X` (select `bool` (`local.isTeamA?`) :`false` _returnvalue_2 :`true` (* _returnvalue_2 -1)) :!label _label)
    (set `local.Y` (`KismetMathLibrary.RandomIntegerInRange` _tileareav_min _tileareav_max))
    (if (== (`KismetArrayLibrary.Array_Find` (`local.Temp`) (`KismetMathLibrary.MakeVector2D` (`KismetMathLibrary.Conv_IntToDouble` (`local.X`)) (`KismetMathLibrary.Conv_IntToDouble` (`local.Y`)))) -1)
      (bind _returnvalue_3 (`|SpawnActorFromClass` (select `/Game/Blueprints/Characters/E_AgentClass` (`local.Agent Class Enum`) :`NewEnumerator0` "/Game/Blueprints/Characters/BP_Swordsman.BP_Swordsman_C" :`NewEnumerator1` "/Game/Blueprints/Characters/BP_Shooter.BP_Shooter_C" :`NewEnumerator2` "/Game/Blueprints/Characters/BP_StaffFighter.BP_StaffFighter_C" :!type "/Game/Blueprints/Characters/BP_BaseAgent Class Reference") (`KismetMathLibrary.MakeTransform` (`KismetMathLibrary.MakeVector` (+ (`self.GetValueFromTileIndex` (`local.X`)) (.x (.location _returnvalue))) (+ (`self.GetValueFromTileIndex` (`local.Y`)) (.y (.location _returnvalue))) (+ (.z (.location _returnvalue)) 100.0)) (`KismetMathLibrary.MakeRotator` (.roll (.rotation _returnvalue)) (.pitch (.rotation _returnvalue)) (+ (.yaw (.rotation _returnvalue)) (select `bool` (`local.isTeamA?`) :`false` 180.0 :!type "Float (single-precision)")))) "AdjustIfPossibleButDontSpawnIfColliding" "OverrideRootScale" null self (select `/Game/Blueprints/Characters/E_AgentClass` (`local.Agent Class Enum`) :`NewEnumerator0` (`/Game/Blueprints/GI_Main.SwordsManKromosom` _gi) :`NewEnumerator1` (`/Game/Blueprints/GI_Main.ShooterKromosom` _gi) :`NewEnumerator2` (`/Game/Blueprints/GI_Main.StaffFighterKromosom` _gi)) null))
      (`/Engine/EditorBlueprintResources/StandardMacros.IsValid` _returnvalue_3
        (:`Is Valid`
          (set `local.Agent` _returnvalue_3)
          (`KismetArrayLibrary.Array_AddUnique` (`local.Temp`) (`KismetMathLibrary.MakeVector2D` (`KismetMathLibrary.Conv_IntToDouble` (`local.X`)) (`KismetMathLibrary.Conv_IntToDouble` (`local.Y`))))
          (`KismetArrayLibrary.Array_AddUnique` (select `bool` (`local.isTeamA?`) :`false` (`self.TeamsB`) :`true` (`self.TeamsA`)) _agent)
          (`/Game/Blueprints/Characters/BP_BaseAgent.Event Spawn` _agent false)
          (if (`local.isTeamA?`)
            (set `self.MaxHpA` (+ (`self.MaxHpA`) _maxhp))
            (else
              (set `self.MaxHpB` (+ _maxhp (`self.MaxHpB`))))))
        (:`Is Not Valid`
          (`KismetSystemLibrary.PrintString` "Actor cant spawned" false)))
      (else
        (goto _label))))
  (return))

(fn `SpawnAgent4Training`
  (params (`isTeamA?` :type Boolean))
  (locals (Agent :type "/Game/Blueprints/Characters/BP_BaseAgent Object Reference") (Temp :type "Array of Vector2D Structure") (X :type Integer) (Y :type Integer :default 0) (`Agent Class Enum` :type "/Game/Blueprints/Characters/E_AgentClass Enum"))
  (bind _agent (`local.Agent`))
  (bind (_tileareav_min _tileareav_max) (break `/Game/Blueprints/Property/S_Range` (`self.TileAreaV`)))
  (bind _returnvalue (`SceneComponent.K2_GetComponentToWorld` (`self.DefaultSceneRoot`)))
  (bind _maxhp (`/Game/Blueprints/Characters/BP_BaseAgent.MaxHp` _agent))
  (bind _value (`BlueprintMapLibrary.Map_Find` (`self.TileAreaHForAgent`) (select `/Game/Blueprints/Characters/E_AgentClass` (`local.Agent Class Enum`) :`NewEnumerator0` "/Game/Blueprints/Characters/BP_Swordsman.BP_Swordsman_C" :`NewEnumerator1` "/Game/Blueprints/Characters/BP_Shooter.BP_Shooter_C" :`NewEnumerator2` "/Game/Blueprints/Characters/BP_StaffFighter.BP_StaffFighter_C" :!type "/Game/Blueprints/Characters/BP_BaseAgent Class Reference")))
  (bind _value_2 (`BlueprintMapLibrary.Map_Find` (`/Game/Blueprints/Property/BP_TrainingManager.Arena` (`self.Manager`)) self))
  (bind _returnvalue_2 (`KismetMathLibrary.RandomIntegerInRange` (break `/Game/Blueprints/Property/S_Range` _value) (`.Max_12_950AF26D437BFC0371E1F1A81C10CB70` (break `/Game/Blueprints/Property/S_Range` _value))))
  (`KismetArrayLibrary.Array_Clear` (`local.Temp`))
  (for _ (range 1 (+ (`self.TeamSize`) 1))
    (set `local.Agent Class Enum` (`KismetArrayLibrary.Array_Random` (`self.Agent Class`)))
    (set `local.X` (select `bool` (`local.isTeamA?`) :`false` _returnvalue_2 :`true` (* _returnvalue_2 -1)) :!label _label)
    (set `local.Y` (`KismetMathLibrary.RandomIntegerInRange` _tileareav_min _tileareav_max))
    (if (== (`KismetArrayLibrary.Array_Find` (`local.Temp`) (`KismetMathLibrary.MakeVector2D` (`KismetMathLibrary.Conv_IntToDouble` (`local.X`)) (`KismetMathLibrary.Conv_IntToDouble` (`local.Y`)))) -1)
      (bind _returnvalue_3 (`|SpawnActorFromClass` (select `/Game/Blueprints/Characters/E_AgentClass` (`local.Agent Class Enum`) :`NewEnumerator0` "/Game/Blueprints/Characters/BP_Swordsman.BP_Swordsman_C" :`NewEnumerator1` "/Game/Blueprints/Characters/BP_Shooter.BP_Shooter_C" :`NewEnumerator2` "/Game/Blueprints/Characters/BP_StaffFighter.BP_StaffFighter_C" :!type "/Game/Blueprints/Characters/BP_BaseAgent Class Reference") (`KismetMathLibrary.MakeTransform` (`KismetMathLibrary.MakeVector` (+ (`self.GetValueFromTileIndex` (`local.X`)) (.x (.location _returnvalue))) (+ (`self.GetValueFromTileIndex` (`local.Y`)) (.y (.location _returnvalue))) (+ (.z (.location _returnvalue)) 100.0)) (`KismetMathLibrary.MakeRotator` (.roll (.rotation _returnvalue)) (.pitch (.rotation _returnvalue)) (+ (.yaw (.rotation _returnvalue)) (select `bool` (`local.isTeamA?`) :`false` 180.0 :!type "Float (single-precision)")))) "AdjustIfPossibleButDontSpawnIfColliding" "OverrideRootScale" null self (select `bool` (`local.isTeamA?`) :`false` (`.KromosomIndexB_17_62ED62454D1F6E3C859F8BBE6430BAB5` (break `/Game/Blueprints/S_TeamPair` _value_2)) :`true` (break `/Game/Blueprints/S_TeamPair` _value_2)) null))
      (`/Engine/EditorBlueprintResources/StandardMacros.IsValid` _returnvalue_3
        (:`Is Valid`
          (set `local.Agent` _returnvalue_3)
          (`KismetArrayLibrary.Array_AddUnique` (`local.Temp`) (`KismetMathLibrary.MakeVector2D` (`KismetMathLibrary.Conv_IntToDouble` (`local.X`)) (`KismetMathLibrary.Conv_IntToDouble` (`local.Y`))))
          (`KismetArrayLibrary.Array_AddUnique` (select `bool` (`local.isTeamA?`) :`false` (`self.TeamsB`) :`true` (`self.TeamsA`)) _agent)
          (`/Game/Blueprints/Characters/BP_BaseAgent.Event Spawn` _agent false)
          (if (`local.isTeamA?`)
            (set `self.MaxHpA` (+ (`self.MaxHpA`) _maxhp))
            (else
              (set `self.MaxHpB` (+ _maxhp (`self.MaxHpB`))))))
        (:`Is Not Valid`
          (`KismetSystemLibrary.PrintString` "Actor cant spawned" false)))
      (else
        (goto _label))))
  (return))

(fn `SpawnItemsBuff`
  (locals (Area :type "TwoVectors Structure") (Item :type "/Game/Blueprints/Property/BP_ItemBuff Object Reference") (MinRange :type "Float (double-precision)" :default -5.0) (MaxRange :type "Float (double-precision)" :default 5.0))
  (bind _tilesize (`self.TileSize`))
  (bind (_tileareav_min _tileareav_max) (break `/Game/Blueprints/Property/S_Range` (`self.TileAreaV`)))
  (bind _returnvalue (`SceneComponent.K2_GetComponentToWorld` (`self.DefaultSceneRoot`)))
  (bind _output_get (set `local.Area` (make `TwoVectors` (`KismetMathLibrary.MakeVector` (+ (* (`local.MinRange`) _tilesize) (.x (.location _returnvalue))) (+ (* _tilesize _tileareav_min) (.y (.location _returnvalue))) (.z (.location _returnvalue))) (`KismetMathLibrary.MakeVector` (+ (* (`local.MaxRange`) _tilesize) (.x (.location _returnvalue))) (+ (* _tileareav_max _tilesize) (.y (.location _returnvalue))) (.z (.location _returnvalue)))) :!label _label))
  (bind _returnvalue_2 (`|SpawnActorFromClass` "/Game/Blueprints/Property/BP_ItemBuff.BP_ItemBuff_C" (`KismetMathLibrary.MakeTransform` (`KismetMathLibrary.MakeVector` (`KismetMathLibrary.RandomFloatInRange` (.x (break `TwoVectors` _output_get)) (.x (`.v2` (break `TwoVectors` _output_get)))) (`KismetMathLibrary.RandomFloatInRange` (.y (break `TwoVectors` _output_get)) (.y (`.v2` (break `TwoVectors` _output_get)))) (`KismetMathLibrary.RandomFloatInRange` (.z (break `TwoVectors` _output_get)) (.z (`.v2` (break `TwoVectors` _output_get))))) (`KismetMathLibrary.MakeRotator` 0.0)) "AdjustIfPossibleButDontSpawnIfColliding" "OverrideRootScale" null null))
  (set `local.Item` _returnvalue_2)
  (bind _item (`local.Item`)
    (:`then`
      (`KismetArrayLibrary.Array_Add` (`self.Items Buff`) _item)
      (return))
    (:`else`
      (goto _label))))

(fn `SpawnTileA`
  (locals (X :type "Float (double-precision)" :default 0.0))
  (bind (_teamatileareah_min _teamatileareah_max) (break `/Game/Blueprints/Property/S_Range` (`self.TeamATileAreaH`)))
  (bind (_tileareav_min _tileareav_max) (break `/Game/Blueprints/Property/S_Range` (`self.TileAreaV`)))
  (for _index (range _teamatileareah_max (+ _teamatileareah_min 1))
    (if (not (== 0 _index))
      (set `local.X` (`self.GetValueFromTileIndex` _index))
      (for _index_2 (range _tileareav_min (+ _tileareav_max 1))
        (if (not (== 0 _index_2))
          (bind _returnvalue (`|SpawnActorFromClass` "/Game/Blueprints/Property/BP_Tile.BP_Tile_C" (`KismetMathLibrary.MakeTransform` (`KismetMathLibrary.MakeVector` (`local.X`) (`self.GetValueFromTileIndex` _index_2))) "AlwaysSpawn" "OverrideRootScale" null null))
          (`KismetArrayLibrary.Array_Add` (`self.Tiles`) _returnvalue)
          (`self.K2_AttachToComponent` _returnvalue (`self.Preparation`) "None" "KeepRelative" "KeepRelative" "KeepRelative" true)))))
  (return))

(fn `UserConstructionScript`)