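; BP_ItemBuff is a pickup actor that grants a temporary power and movement speed buff to an agent that touches it.
; A sphere collision overlap casts to BP_BaseAgent, calls the agent's PowerUp and MSpeedUp with a fixed amount and duration, then destroys the pickup.
; Each tick spins the item mesh around its yaw axis at a frame-rate-independent speed.
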(event `self.ReceiveTick`
  (params (DeltaSeconds :type "Float (single-precision)"))
  (`self.Anim`))

(event `self.SphereCol.OnComponentBeginOverlap`
  (params (OverlappedComponent :type "PrimitiveComponent Object Reference") (OtherActor :type "Actor Object Reference") (OtherComp :type "PrimitiveComponent Object Reference") (OtherBodyIndex :type Integer) (bFromSweep :type Boolean) (SweepResult :type "HitResult Structure (by ref)"))
  (bind _asbp_base_agent (cast `/Game/Blueprints/Characters/BP_BaseAgent` OtherActor))
  (`self.BuffActivated` _asbp_base_agent)
  (`self.K2_DestroyActor`))

(event `BuffActivated`
  (params (Agent :type "/Game/Blueprints/Characters/BP_BaseAgent Object Reference"))
  (`/Game/Blueprints/Characters/BP_BaseAgent.Power Up` Agent 0.25 true 15.0)
  (`/Game/Blueprints/Characters/BP_BaseAgent.MSpeed Up` Agent 0.25 true 15.0))

(event `Anim`
  (`SceneComponent.K2_AddRelativeRotation` (`self.Item`) (`KismetMathLibrary.MakeRotator` 0.0 0.0 (* (`GameplayStatics.GetWorldDeltaSeconds`) 90.0)) false false))

(fn `UserConstructionScript`)