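; Training manager that evolves combat agent chromosomes through repeated team battles, muting master audio during runs.
; It seeds first generations through GI_Main, then each iteration spawns an arena grid and randomly pairs the first agent class's chromosomes.
; Tied pairs are blacklisted from rematches, with reshuffles on conflicts, until one loses.
; Arenas report scores and wins via FightFinished; once all finish, the next iteration starts, saving results after the iteration limit.
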(event `self.ReceiveBeginPlay`
  (for _array_element (`self.ClassAgent`)
    (`/Game/Blueprints/GI_Main.Generate First Generation` (`self.GetGI`) _array_element 32))
  (`GameplayStatics.SetSoundMixClassOverride` "/Game/Sounds/MasterSoundMix.MasterSoundMix" "/Game/Sounds/SC_Master.SC_Master" 0.0)
  (`GameplayStatics.PushSoundMixModifier` "/Game/Sounds/MasterSoundMix.MasterSoundMix")
  (`self.Start Next Training`))

(event `Start Next Training`
  (bind _gi_main (`self.GetGI`))
  (bind _classagent (`self.ClassAgent`))
  (bind _curtrainingiteration (`/Game/Blueprints/GI_Main.CurTrainingIteration` (`self.GetGI`)))
  (if (<= _curtrainingiteration (`self.MaxIterasi`))
    (`/Engine/EditorBlueprintResources/StandardMacros.IncrementInt` _curtrainingiteration
      (:`  `
        (`self.Spawn Arena` _classagent 4 4 5)
        (`self.Generate Battle List` (select `/Game/Blueprints/Characters/E_AgentClass` (`|GetArrayItem` _classagent) :`NewEnumerator0` (`/Game/Blueprints/GI_Main.TSwordsManKromosom` _gi_main) :`NewEnumerator1` (`/Game/Blueprints/GI_Main.TShooterKromosom` _gi_main) :`NewEnumerator2` (`/Game/Blueprints/GI_Main.TStaffFighterKromosom` _gi_main)))
        (bind _keys (`BlueprintMapLibrary.Map_Keys` (`self.Arena`)))
        (for _array_element _keys
          (`/Engine/EditorBlueprintResources/StandardMacros.IsValid` _array_element
            (:`Is Valid`
              (`/Game/Blueprints/Property/BP_Arena.Start Training` _array_element))))))
    (else
      ;[1 1 1] Training Finished
      (`KismetSystemLibrary.PrintString` "Training Finished")
      (for _array_element_2 (`self.ClassAgent`)
        (`/Game/Blueprints/GM_Main.Save_Training_Result` (`/Game/Blueprints/GI_Main.Get_GM` (`self.GetGI`)) _array_element_2)))))

(fn `AddToBlacklist`
  (params (Id_Pair :type "/Game/Blueprints/Property/S_IdPair Structure"))
  (locals (A :type Integer) (B :type Integer))
  (bind (_id_a _id_b) (break `/Game/Blueprints/Property/S_IdPair` Id_Pair))
  (bind _blacklist (`self.Blacklist`))
  (bind (_value _returnvalue) (`BlueprintMapLibrary.Map_Find` _blacklist (`local.B`)))
  (bind (_value_2 _returnvalue_2) (`BlueprintMapLibrary.Map_Find` _blacklist (`local.A`)))
  (set `local.A` _id_a)
  (set `local.B` _id_b)
  (if _returnvalue_2
    (`KismetArrayLibrary.Array_Add` (break `/Game/Blueprints/Property/S_ArrInt` _value_2) (`local.B`))
    (elif _returnvalue
      (`KismetArrayLibrary.Array_Add` (break `/Game/Blueprints/Property/S_ArrInt` _value) (`local.A`))
      (else
        (`BlueprintMapLibrary.Map_Add` _blacklist (`local.A`) (make `/Game/Blueprints/Property/S_ArrInt` (`|MakeArray` (`local.B`)))))))
  (return))

(fn `FightFinished`
  (params (Arena :type "/Game/Blueprints/Property/BP_Arena Object Reference") (State :type "/Game/Blueprints/Property/E_BattleState Enum" :default "NewEnumerator0"))
  (locals (TeamA :type "/Game/Blueprints/Characters/BT/S_Kromosom Structure") (TeamB :type "/Game/Blueprints/Characters/BT/S_Kromosom Structure"))
  (bind _gi_main (`self.GetGI`))
  (bind _gi_main_2 (`self.GetGI`))
  (bind _arena (`local.Arena`))
  (bind _teama (`local.TeamA`))
  (bind _teamb (`local.TeamB`))
  (bind _teama_2 (`local.TeamA`))
  (bind _teamb_2 (`local.TeamB`))
  (bind _value (`BlueprintMapLibrary.Map_Find` (`self.Arena`) _arena))
  (set `local.TeamA` (break `/Game/Blueprints/S_TeamPair` _value))
  (set `local.TeamB` (`.KromosomIndexB_17_62ED62454D1F6E3C859F8BBE6430BAB5` (break `/Game/Blueprints/S_TeamPair` _value)))
  (`/Game/Blueprints/GI_Main.Add Bonus Skor` _gi_main (`local.TeamA`) _arena true)
  (`/Game/Blueprints/GI_Main.Add Bonus Skor` _gi_main (`local.TeamB`) _arena false)
  (switch `/Game/Blueprints/Property/E_BattleState` (`local.State`)
    (:`NewEnumerator0`
      (return))
    (:`NewEnumerator1`
      (return))
    (:`NewEnumerator2`
      (`self.RemoveFromBlacklist` (make `/Game/Blueprints/Property/S_IdPair` (`.Id_11_37E72B9C49D3D54F99EF61A75A7FFB8F` (break `/Game/Blueprints/Characters/BT/S_Kromosom` _teama)) (`.Id_11_37E72B9C49D3D54F99EF61A75A7FFB8F` (break `/Game/Blueprints/Characters/BT/S_Kromosom` _teamb))))
      (`/Game/Blueprints/GI_Main.Fight Win` _gi_main_2 _teama _teamb))
    (:`NewEnumerator3`
      (`self.RemoveFromBlacklist` (make `/Game/Blueprints/Property/S_IdPair` (`.Id_11_37E72B9C49D3D54F99EF61A75A7FFB8F` (break `/Game/Blueprints/Characters/BT/S_Kromosom` _teamb_2)) (`.Id_11_37E72B9C49D3D54F99EF61A75A7FFB8F` (break `/Game/Blueprints/Characters/BT/S_Kromosom` _teama_2))))
      (`/Game/Blueprints/GI_Main.Fight Win` _gi_main_2 _teamb_2 _teama_2))
    (:`NewEnumerator4`
      (`self.AddToBlacklist` (make `/Game/Blueprints/Property/S_IdPair` (`.Id_11_37E72B9C49D3D54F99EF61A75A7FFB8F` (break `/Game/Blueprints/Characters/BT/S_Kromosom` (`local.TeamA`))) (`.Id_11_37E72B9C49D3D54F99EF61A75A7FFB8F` (break `/Game/Blueprints/Characters/BT/S_Kromosom` (`local.TeamB`)))))))
  (`/Game/Blueprints/Property/BP_Arena.On Battle End` _arena)
  (bind _result (`/Engine/EditorBlueprintResources/StandardMacros.IncrementInt` (`self.TempCountArena`))
    (:`  `
      (if (== _result (`BlueprintMapLibrary.Map_Length` (`self.Arena`)))
        (set `self.TempCountArena` 0)
        (`self.Start Next Training`)
        (return)))))

(fn `Generate Battle List`
  (params (`Team List` :type "Array of /Game/Blueprints/Characters/BT/S_Kromosom Structure"))
  (locals (`Team A` :type "/Game/Blueprints/Characters/BT/S_Kromosom Structure") (`Team B` :type "/Game/Blueprints/Characters/BT/S_Kromosom Structure") (`Temp Team List` :type "Array of /Game/Blueprints/Characters/BT/S_Kromosom Structure") (TempInt :type Integer) (LoopLimit :type Integer))
  (bind _arena (`self.Arena`))
  (bind _team_list (`local.Team List`))
  (bind _team_list_2 (`local.Team List`))
  (bind _returnvalue (/ (`KismetArrayLibrary.Array_Length` _team_list_2) 2))
  (for _ (range (+ (`local.LoopLimit`) 1))
    (`KismetArrayLibrary.Array_Shuffle` _team_list_2)
    (set `local.TempInt` _returnvalue)
    (for _index (range _returnvalue)
      (set `local.Team A` (`|GetArrayItem` _team_list _index))
      (set `local.Team B` (`|GetArrayItem` _team_list (+ _index (`local.TempInt`))))
      (if (`self.OnBlacklist?` (make `/Game/Blueprints/Property/S_IdPair` (`.Id_11_37E72B9C49D3D54F99EF61A75A7FFB8F` (break `/Game/Blueprints/Characters/BT/S_Kromosom` (`local.Team A`))) (`.Id_11_37E72B9C49D3D54F99EF61A75A7FFB8F` (break `/Game/Blueprints/Characters/BT/S_Kromosom` (`local.Team B`)))))
        ;[1 1 1] Re-Generate
        (`/Engine/EditorBlueprintResources/StandardMacros.IncrementInt` (`local.LoopLimit`)
          (:`  `
            (break)))
        (else
          (bind _keys (`BlueprintMapLibrary.Map_Keys` _arena))
          (`BlueprintMapLibrary.Map_Add` _arena (`|GetArrayItem` _keys _index) (make `/Game/Blueprints/S_TeamPair` (`local.Team A`) (`local.Team B`)))))))
  (return))

(fn `GetGI`
  (returns (`GI Main` :type "/Game/Blueprints/GI_Main Object Reference"))
  (`self.GI Main`
    (:`then`
      _)
    (:`else`
      (bind _asgi_main (cast `/Game/Blueprints/GI_Main` (`GameplayStatics.GetGameInstance`)))
      (set `self.GI Main` _asgi_main)))
  (return (`self.GI Main`)))

(fn `GetHUD`
  (returns (HUD :type "/Game/Blueprints/HUD_Main Object Reference"))
  (`self.HUD`
    (:`then`
      _)
    (:`else`
      (bind _ashud_main (cast `/Game/Blueprints/HUD_Main` (`PlayerController.GetHUD` (`GameplayStatics.GetPlayerController` 0)))
        (:`then`
          (set `self.HUD` _ashud_main))
        (:`CastFailed`
          _))))
  (return (`self.HUD`)))

(fn `OnBlacklist?`
  (params (Id_Pair :type "/Game/Blueprints/Property/S_IdPair Structure"))
  (returns (Value :type Boolean))
  (bind _blacklist (`self.Blacklist`))
  (bind _id_pair_id_a (break `/Game/Blueprints/Property/S_IdPair` (`local.Id_Pair`)))
  (bind _id_pair_id_a_2 (break `/Game/Blueprints/Property/S_IdPair` (`local.Id_Pair`)))
  (bind (_id_pair_id_a_3 _id_pair_id_b) (break `/Game/Blueprints/Property/S_IdPair` (`local.Id_Pair`)))
  (bind (_id_a _id_b) (break `/Game/Blueprints/Property/S_IdPair` (`local.Id_Pair`)))
  (bind (_value _returnvalue) (`BlueprintMapLibrary.Map_Find` _blacklist _id_pair_id_a_2))
  (bind (_value_2 _returnvalue_2) (`BlueprintMapLibrary.Map_Find` _blacklist _id_pair_id_b))
  (if (== _id_a _id_b)
    (return true)
    (else
      (if _returnvalue
        (for _array_element (`.Member_3_D209499E49F9C06C66CB0EAB2589A39C` (break `/Game/Blueprints/Property/S_ArrInt` _value))
          (if (== _array_element _id_pair_id_b)
            (return true))))
      (if _returnvalue_2
        (for _array_element_2 (`.Member_3_D209499E49F9C06C66CB0EAB2589A39C` (break `/Game/Blueprints/Property/S_ArrInt` _value_2))
          (if (== _array_element_2 _id_pair_id_a)
            (return true))))
      (return false))))

(fn `RemoveFromBlacklist`
  (params (Id_Pair :type "/Game/Blueprints/Property/S_IdPair Structure"))
  (bind _blacklist (`self.Blacklist`))
  (bind (_id_pair_id_a _id_pair_id_b) (break `/Game/Blueprints/Property/S_IdPair` (`local.Id_Pair`)))
  (bind (_id_pair_id_a_2 _id_pair_id_b_2) (break `/Game/Blueprints/Property/S_IdPair` (`local.Id_Pair`)))
  (bind _returnvalue (`BlueprintMapLibrary.Map_Remove` _blacklist _id_pair_id_b_2))
  (if _returnvalue
    (`KismetSystemLibrary.PrintString` (`KismetStringLibrary.Concat_StrStr` (`KismetStringLibrary.Conv_IntToString` _id_pair_id_b_2) " - removed from blaclist"))
    (bind _values (`BlueprintMapLibrary.Map_Values` _blacklist)))
  (for _array_element _values
    (bind _returnvalue_2 (`KismetArrayLibrary.Array_RemoveItem` (break `/Game/Blueprints/Property/S_ArrInt` _array_element) _id_pair_id_b))
    (if _returnvalue_2
      (`KismetSystemLibrary.PrintString` "removed from blaclist value")))
  (return))

(fn `Spawn Arena`
  (params (`Agent Class_` :type "Array of /Game/Blueprints/Characters/E_AgentClass Enum") (`Amount X` :type Integer) (`Amount Y` :type Integer) (TeamSize :type Integer))
  (`BlueprintMapLibrary.Map_Clear` (`self.Arena`))
  (for _index (range (* `Amount X` `Amount Y`))
    (bind _returnvalue (`|SpawnActorFromClass` "/Game/Blueprints/Property/BP_Arena.BP_Arena_C" (`KismetMathLibrary.MakeTransform` (`KismetMathLibrary.MakeVector` (* (mod _index (`local.Amount X`)) 10000) (* (/ _index (`local.Amount Y`)) 10000))) "Undefined" "OverrideRootScale" null self _index TeamSize (`local.Agent Class_`) true null))
    (`BlueprintMapLibrary.Map_Add` (`self.Arena`) _returnvalue))
  (return))

(fn `UserConstructionScript`)