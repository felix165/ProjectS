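; BP_Info is a debug actor that exposes the chromosome data of the Swordsman, Shooter and StaffFighter classes held in GI_Main.
; Every Tick it copies each class's T, A and B chromosome variables from the game instance into its own.
; PrintKromosome prints each class's T array through the game mode's PrintKromosomInfo, and TryRandom prints a ConeRandom sample.
; Cached getters resolve the game instance and HUD, though the HUD goes unused here.
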(event `self.ReceiveBeginPlay`)

(event `self.ReceiveTick`
  (params (DeltaSeconds :type "Float (single-precision)"))
  (bind _gi (`self.Get_GI`))
  (set `self.TSwords Man Kromosom` (`/Game/Blueprints/GI_Main.TSwordsManKromosom` _gi))
  (set `self.Swords Man Kromosom A` (`/Game/Blueprints/GI_Main.SwordsManKromosom_A` _gi))
  (set `self.Swords Man Kromosom B` (`/Game/Blueprints/GI_Main.SwordsManKromosom_B` _gi))
  (set `self.TShooter Kromosom` (`/Game/Blueprints/GI_Main.TShooterKromosom` _gi))
  (set `self.Shooter Kromosom A` (`/Game/Blueprints/GI_Main.ShooterKromosom_A` _gi))
  (set `self.Shooter Kromosom B` (`/Game/Blueprints/GI_Main.ShooterKromosom_B` _gi))
  (set `self.TStaff Fighter Kromosom` (`/Game/Blueprints/GI_Main.TStaffFighterKromosom` _gi))
  (set `self.Staff Fighter Kromosom A` (`/Game/Blueprints/GI_Main.StaffFighterKromosom_A` _gi))
  (set `self.Staff Fighter Kromosom B` (`/Game/Blueprints/GI_Main.StaffFighterKromosom_B` _gi)))

(event `Print Kromosome`
  (bind _gi (`self.Get_GI`))
  (bind _gm (`/Game/Blueprints/GI_Main.Get_GM` (`self.Get_GI`)))
  (for _array_element (`/Game/Blueprints/GI_Main.TSwordsManKromosom` _gi)
    (`/Game/Blueprints/GM_Main.Print Kromosom Info` _gm _array_element))
  (`KismetSystemLibrary.PrintString` "***************")
  (for _array_element_2 (`/Game/Blueprints/GI_Main.TShooterKromosom` _gi)
    (`/Game/Blueprints/GM_Main.Print Kromosom Info` _gm _array_element_2))
  (`KismetSystemLibrary.PrintString` "***************")
  (for _array_element_3 (`/Game/Blueprints/GI_Main.TStaffFighterKromosom` _gi)
    (`/Game/Blueprints/GM_Main.Print Kromosom Info` _gm _array_element_3)))

(event `TryRandom`
  (`KismetSystemLibrary.PrintString` (`KismetStringLibrary.Conv_DoubleToString` (`/Game/Blueprints/BlueprintLibrary/Function/BPF_ConeRandom.Cone Random` 0.0 1000.0))))

(fn `Get_GI`
  (returns (GI :type "/Game/Blueprints/GI_Main Object Reference"))
  (`self.GI`
    (:`then`
      _)
    (:`else`
      (bind _asgi_main (cast `/Game/Blueprints/GI_Main` (`GameplayStatics.GetGameInstance`))
        (:`then`
          (set `self.GI` _asgi_main))
        (:`CastFailed`
          _))))
  (return (`self.GI`)))

(fn `GetHUD`
  (returns (HUD :type "/Game/Blueprints/HUD_Main Object Reference"))
  (`self.HUD`
    (:`then`
      _)
    (:`else`
      (bind _ashud_main (cast `/Game/Blueprints/HUD_Main` (`PlayerController.GetHUD` (`GameplayStatics.GetPlayerController` 0)))
        (:`then`
          (set `self.HUD` _ashud_main))
        (:`CastFailed`
          _))))
  (return (`self.HUD`)))

(fn `UserConstructionScript`)