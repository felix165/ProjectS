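; BP_Arena_InGame_1 is a battle arena that runs one fight, in either training or player-facing mode, and handles its result.
; Tick refreshes the arena's state and timer text, accumulates time and checks battle state during combat.
; On a win or tie it fires once: training reports to the Manager, otherwise wins update HUD and training data, and item spawning stops.
; Surrender forces a B win that skips the training-data update outside training.
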(event `self.ReceiveTick`
  (params (DeltaSeconds :type "Float (single-precision)"))
  (bind _hud (`self.GetHUD`))
  (bind _curtime (`self.CurTime`))
  (bind _battlestate (`self.BattleState`))
  (bind _gm (`/Game/Blueprints/GI_Main.Get_GM` (`self.GetGI`)))
  (`TextRenderComponent.K2_SetText` (`self.State`) (`KismetTextLibrary.Conv_StringToText` (`KismetStringLibrary.Concat_StrStr` "Arena - " (`KismetStringLibrary.Conv_IntToString` (`self.IndexArena`)) " \n" (`|GetEnumeratorNameAsString` _battlestate))))
  (`TextRenderComponent.K2_SetText` (`self.Time`) (`KismetTextLibrary.Conv_StringToText` (`KismetStringLibrary.Concat_StrStr` (`KismetStringLibrary.Conv_IntToString` (/ (`KismetMathLibrary.FTrunc` _curtime) 60)) " : " (`KismetStringLibrary.Conv_IntToString` (mod (`KismetMathLibrary.FTrunc` _curtime) 60)))))
  (switch `/Game/Blueprints/Property/E_BattleState` _battlestate
    (:`NewEnumerator1`
      (set `self.CurTime` (+ (`self.CurTime`) (`GameplayStatics.GetWorldDeltaSeconds`)))
      (`self.CheckBattleState`))
    (:`NewEnumerator2`
      (`/Engine/EditorBlueprintResources/StandardMacros.DoOnce` false :!label _label
        (:`Completed`
          (if (`self.isTraining?`)
            (`/Game/Blueprints/Property/BP_TrainingManager.FightFinished` (`self.Manager`) self _battlestate)
            (else
              (switch `/Game/Blueprints/Property/E_BattleState` _battlestate
                (:`NewEnumerator2`
                  (`/Game/Blueprints/HUD_Main.BattleEnd` _hud true)
                  (`/Game/Blueprints/GM_Main.Update Training Data` _gm true))
                (:`NewEnumerator3`
                  (`/Game/Blueprints/HUD_Main.BattleEnd` _hud false)
                  (if (not (`self.IsSurrender`))
                    (`/Game/Blueprints/GM_Main.Update Training Data` _gm false))))))
          (`KismetSystemLibrary.K2_ClearAndInvalidateTimerHandle` (`self.SpawnItemHandle`)))))
    (:`NewEnumerator3`
      (goto _label))
    (:`NewEnumerator4`
      (goto _label))))

(event `Surrender`
  (set `self.IsSurrender` true)
  (set `self.BattleState` "NewEnumerator3"))

(fn `UserConstructionScript`
  (`parent.UserConstructionScript`))