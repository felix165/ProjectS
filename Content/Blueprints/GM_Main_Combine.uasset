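; Game mode that combines saved training results for the Swordsman, Shooter and Staff-Fighter agents into one save slot.
; On BeginPlay it cycles through the agents, async-loading each one's source slot from FromSlot.
; Each load copies one hardcoded-index chromosome into that agent's Game Instance array, then advances to the next.
; After three loads, the LoadFinished event triggers a save of all results to ToSlot.
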(event `Next`
  (switch `/Game/Blueprints/Characters/E_AgentClass` (`self.Agent`)
    (:`NewEnumerator0`
      (set `self.Agent` "NewEnumerator1"))
    (:`NewEnumerator1`
      (set `self.Agent` "NewEnumerator2"))
    (:`NewEnumerator2`
      (set `self.Agent` "NewEnumerator0")))
  (set `self.SlotName` (`BlueprintMapLibrary.Map_Find` (`self.From Slot`) (`self.Agent`)))
  (`self.Load_Training_Result`))

(event `self.ReceiveBeginPlay`
  (`parent.ReceiveBeginPlay`)
  (`self.Next`)
  (add `self.Load Finished` (delegate `Save`)))

(event `Save` :!signature `self.Load Finished`
  (params (isSuccess :type Boolean))
  (`KismetSystemLibrary.PrintString` "Load all Success" isSuccess isSuccess)
  (set `self.SlotName` (`self.To Slot`))
  (`self.Save_Training_Result` "NewEnumerator0" true))

(event `self.Load_Training_Result`
  (bind _returnvalue (`self.GetSaveSlotName`))
  (bind _gi_main (`self.GetGI`))
  (bind _returnvalue_2 (`GameplayStatics.DoesSaveGameExist` _returnvalue))
  (if _returnvalue_2
    (bind _savegame (`AsyncActionHandleSaveGame.AsyncLoadGameFromSlot` _returnvalue)
      (:`Completed`
        (bind _assg_training_result (cast `/Game/Blueprints/SG_TrainingResult` _savegame))
        (bind _output_get (set `self.SaveObject` _assg_training_result))
        (switch `/Game/Blueprints/Characters/E_AgentClass` (`self.Agent`)
          (:`NewEnumerator0`
            (set `/Game/Blueprints/GI_Main.TSwordsManKromosom` (`|MakeArray` (`|GetArrayItem` (`/Game/Blueprints/SG_TrainingResult.TSwordsManKromosom` _output_get) 27)) _gi_main))
          (:`NewEnumerator1`
            (set `/Game/Blueprints/GI_Main.TShooterKromosom` (`|MakeArray` (`|GetArrayItem` (`/Game/Blueprints/SG_TrainingResult.TShooterKromosom` _output_get) 29)) _gi_main))
          (:`NewEnumerator2`
            (set `/Game/Blueprints/GI_Main.TStaffFighterKromosom` (`|MakeArray` (`|GetArrayItem` (`/Game/Blueprints/SG_TrainingResult.TStaffFighterKromosom` _output_get) 30)) _gi_main)))
        (bind _result (`/Engine/EditorBlueprintResources/StandardMacros.IncrementInt` (`self.Counter`))
          (:`  `
            (if (== _result 3)
              (`self.Load Finished` true)
              (else
                (`self.Next`)))))))))

(fn `UserConstructionScript`
  (`parent.UserConstructionScript`))