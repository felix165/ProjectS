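; GM_Main_Migrate is a utility game mode that copies saved training results from one save slot to another when play begins.
; After the parent BeginPlay, it points SlotName at FromSlot and loads the training result.
; It then switches SlotName to ToSlot and saves with SaveAll enabled.
; Tick is disabled, and the construction script only calls its parent.
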(event `self.ReceiveBeginPlay`
  (`parent.ReceiveBeginPlay`)
  (set `self.SlotName` (`self.From Slot`))
  (`self.Load_Training_Result`)
  (set `self.SlotName` (`self.To Slot`))
  (`self.Save_Training_Result` "NewEnumerator0" true))

(fn `UserConstructionScript`
  (`parent.UserConstructionScript`))