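; Game mode for a genetic-algorithm agent training match, handling level travel, pause, cycling game speed and chromosome persistence.
; Saving writes score-sorted Swordsman, Shooter and Staff-Fighter chromosome pools from the game instance to a save slot, per class or all.
; Loading restores those pools asynchronously, then seeds both teams from random top-ten picks, optionally bred through crossover-mutation.
; A missing slot on load gets an empty save instead.
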(event `self.ReceiveBeginPlay`
  (set `PlayerController.bShowMouseCursor` true (`GameplayStatics.GetPlayerController` 0)))

(event `OpenLevel`
  (params (Destination :type "World Soft Object Reference"))
  (`/Game/Blueprints/HUD_Main.CleanViewport` (`self.GetHUD`))
  (`GameplayStatics.OpenLevelBySoftObjectPtr` Destination))

(event `Restart Level`
  (`KismetSystemLibrary.ExecuteConsoleCommand` "RestartLevel" null))

(event `Save_Training_Result`
  (params (`Agent Class` :type "/Game/Blueprints/Characters/E_AgentClass Enum" :default "NewEnumerator0") (`SaveAll?` :type Boolean))
  (bind _hud (`self.GetHUD`))
  (bind _result_ (`self.Filter Chromosome` `Agent Class`))
  (bind _slotname (`self.SlotName`))
  (bind _saveobject (`self.SaveObject`))
  (bind _saveobject_2 (`self.SaveObject`))
  (bind _tshooterkromosom (`/Game/Blueprints/SG_TrainingResult.TShooterKromosom` _saveobject_2))
  (bind _tswordsmankromosom (`/Game/Blueprints/SG_TrainingResult.TSwordsManKromosom` _saveobject))
  (bind _tstafffighterkromosom (`/Game/Blueprints/SG_TrainingResult.TStaffFighterKromosom` _saveobject))
  (bind _tshooterkromosom_2 (`/Game/Blueprints/SG_TrainingResult.TShooterKromosom` _saveobject))
  (bind _tswordsmankromosom_2 (`/Game/Blueprints/SG_TrainingResult.TSwordsManKromosom` _saveobject_2))
  (bind _tstafffighterkromosom_2 (`/Game/Blueprints/SG_TrainingResult.TStaffFighterKromosom` _saveobject_2))
  ;[0 0.192 1] Saving_Event
  (bind _returnvalue (`GameplayStatics.DoesSaveGameExist` _slotname))
  (if _returnvalue
    (bind _returnvalue_2 (`GameplayStatics.LoadGameFromSlot` _slotname))
    (bind _assg_training_result (cast `/Game/Blueprints/SG_TrainingResult` _returnvalue_2))
    (set `self.SaveObject` _assg_training_result)
    (else
      (bind _returnvalue_3 (`GameplayStatics.CreateSaveGameObject` "/Game/Blueprints/SG_TrainingResult.SG_TrainingResult_C"))
      (set `self.SaveObject` _returnvalue_3)))
  (if `SaveAll?`
    (`KismetArrayLibrary.Array_Clear` _tswordsmankromosom_2)
    (`KismetArrayLibrary.Array_Append` _tswordsmankromosom_2 (`self.Filter Chromosome` "NewEnumerator0"))
    (`KismetArrayLibrary.Array_Clear` _tshooterkromosom)
    (`KismetArrayLibrary.Array_Append` _tshooterkromosom (`self.Filter Chromosome` "NewEnumerator1"))
    (`KismetArrayLibrary.Array_Clear` _tstafffighterkromosom_2)
    (`KismetArrayLibrary.Array_Append` _tstafffighterkromosom_2 (`self.Filter Chromosome` "NewEnumerator2"))
    (bind (_savegame _bsuccess) (`AsyncActionHandleSaveGame.AsyncSaveGameToSlot` (`self.SaveObject`) (`self.SlotName`))
      (:`Completed`
        (`/Game/Blueprints/HUD_Main.SaveCompleted` _hud _bsuccess)))
    (else
      (switch `/Game/Blueprints/Characters/E_AgentClass` `Agent Class`
        (:`NewEnumerator0`
          (`KismetArrayLibrary.Array_Clear` _tswordsmankromosom)
          (`KismetArrayLibrary.Array_Append` _tswordsmankromosom _result_))
        (:`NewEnumerator1`
          (`KismetArrayLibrary.Array_Clear` _tshooterkromosom_2)
          (`KismetArrayLibrary.Array_Append` _tshooterkromosom_2 _result_))
        (:`NewEnumerator2`
          (`KismetArrayLibrary.Array_Clear` _tstafffighterkromosom)
          (`KismetArrayLibrary.Array_Append` _tstafffighterkromosom _result_)))
      (bind (_savegame_2 _bsuccess_2) (`AsyncActionHandleSaveGame.AsyncSaveGameToSlot` (`self.SaveObject`) (`self.SlotName`))
        (:`Completed`
          (`/Game/Blueprints/HUD_Main.SaveCompleted` _hud _bsuccess_2))))))

(event `Load_Training_Result`
  (bind _gi_main (`self.GetGI`))
  (bind _gi_main_2 (`self.GetGI`))
  (bind _gi_main_3 (`self.GetGI`))
  (bind _slotname (`self.SlotName`))
  (bind _isdocrossover (`self.isDoCrossover`))
  (bind _isdocrossover_2 (`self.isDoCrossover`))
  ;[0 0.192 1] Saving_Event
  (bind _returnvalue (`GameplayStatics.DoesSaveGameExist` _slotname))
  (if _returnvalue
    (bind _savegame (`AsyncActionHandleSaveGame.AsyncLoadGameFromSlot` _slotname)
      (:`Completed`
        (bind _assg_training_result (cast `/Game/Blueprints/SG_TrainingResult` _savegame))
        (bind _output_get (set `self.SaveObject` _assg_training_result))
        (set `/Game/Blueprints/GI_Main.TSwordsManKromosom` (`/Game/Blueprints/SG_TrainingResult.TSwordsManKromosom` _output_get) _gi_main_3)
        (set `/Game/Blueprints/GI_Main.TShooterKromosom` (`/Game/Blueprints/SG_TrainingResult.TShooterKromosom` _output_get) _gi_main_3)
        (set `/Game/Blueprints/GI_Main.TStaffFighterKromosom` (`/Game/Blueprints/SG_TrainingResult.TStaffFighterKromosom` _output_get) _gi_main_3)
        ;;[1 1 1] Team A
        (bind _result (`self.Random Chromosome` (`/Game/Blueprints/GI_Main.TSwordsManKromosom` _gi_main_2) _isdocrossover_2))
        (set `/Game/Blueprints/GI_Main.SwordsManKromosom_A` _result _gi_main_3)
        (bind _result_2 (`self.Random Chromosome` (`/Game/Blueprints/GI_Main.TShooterKromosom` _gi_main_2) _isdocrossover_2))
        (set `/Game/Blueprints/GI_Main.ShooterKromosom_A` _result_2 _gi_main_3)
        (bind _result_3 (`self.Random Chromosome` (`/Game/Blueprints/GI_Main.TStaffFighterKromosom` _gi_main_2) _isdocrossover_2))
        (set `/Game/Blueprints/GI_Main.StaffFighterKromosom_A` _result_3 _gi_main_3)
        ;;[1 1 1] Team B
        (bind _result_4 (`self.Random Chromosome` (`/Game/Blueprints/GI_Main.TSwordsManKromosom` _gi_main) _isdocrossover))
        (set `/Game/Blueprints/GI_Main.SwordsManKromosom_B` _result_4 _gi_main)
        (bind _result_5 (`self.Random Chromosome` (`/Game/Blueprints/GI_Main.TShooterKromosom` _gi_main) _isdocrossover))
        (set `/Game/Blueprints/GI_Main.ShooterKromosom_B` _result_5 _gi_main)
        (bind _result_6 (`self.Random Chromosome` (`/Game/Blueprints/GI_Main.TStaffFighterKromosom` _gi_main) _isdocrossover))
        (set `/Game/Blueprints/GI_Main.StaffFighterKromosom_B` _result_6 _gi_main)
        (`KismetSystemLibrary.PrintString` "Load Finished")))
    (else
      (`KismetSystemLibrary.PrintString` "Save Slot doesnt exist" true true (struct :`G` 0.66 :`B` 1.0 :`A` 1.0) 2.0 "Save")
      (bind _returnvalue_2 (`GameplayStatics.CreateSaveGameObject` "/Game/Blueprints/SG_TrainingResult.SG_TrainingResult_C"))
      (`/Engine/EditorBlueprintResources/StandardMacros.IsValid` _returnvalue_2
        (:`Is Valid`
          (`AsyncActionHandleSaveGame.AsyncSaveGameToSlot` _returnvalue_2 (`self.SlotName`)
            (:`Completed`
              (`KismetSystemLibrary.PrintString` "create Save success"))))
        (:`Is Not Valid`
          (`KismetSystemLibrary.PrintString` "create save failed"))))))

(fn `Filter Chromosome`
  (params (Index :type "/Game/Blueprints/Characters/E_AgentClass Enum" :default "NewEnumerator0"))
  (returns (Result_ :type "Array of /Game/Blueprints/Characters/BT/S_Kromosom Structure"))
  (bind _gi_main (`self.GetGI`))
  (bind _result (`/Game/Blueprints/GI_Main.Sort Chromosome by Score` _gi_main (select `/Game/Blueprints/Characters/E_AgentClass` Index :`NewEnumerator0` (`/Game/Blueprints/GI_Main.TSwordsManKromosom` _gi_main) :`NewEnumerator1` (`/Game/Blueprints/GI_Main.TShooterKromosom` _gi_main) :`NewEnumerator2` (`/Game/Blueprints/GI_Main.TStaffFighterKromosom` _gi_main))))
  (return _result))

(fn `GetGI`
  (returns (`GI Main` :type "/Game/Blueprints/GI_Main Object Reference"))
  (`self.GI Main`
    (:`then`
      _)
    (:`else`
      (bind _asgi_main (cast `/Game/Blueprints/GI_Main` (`GameplayStatics.GetGameInstance`)))
      (set `self.GI Main` _asgi_main)))
  (return (`self.GI Main`)))

(fn `GetHUD`
  (returns (HUD :type "/Game/Blueprints/HUD_Main Object Reference"))
  (`self.HUD`
    (:`then`
      _)
    (:`else`
      (bind _ashud_main (cast `/Game/Blueprints/HUD_Main` (`PlayerController.GetHUD` (`GameplayStatics.GetPlayerController` 0)))
        (:`then`
          (set `self.HUD` _ashud_main))
        (:`CastFailed`
          _))))
  (return (`self.HUD`)))

(fn `Random Chromosome`
  (params (TargetArray :type "Array of /Game/Blueprints/Characters/BT/S_Kromosom Structure (by ref)") (`Do Crossover?` :type Boolean))
  (returns (Result :type "/Game/Blueprints/Characters/BT/S_Kromosom Structure"))
  (locals (tempA :type "/Game/Blueprints/Characters/BT/S_Kromosom Structure") (tempB :type "/Game/Blueprints/Characters/BT/S_Kromosom Structure") (TempArray :type "Array of /Game/Blueprints/Characters/BT/S_Kromosom Structure"))
  (bind _temparray (`local.TempArray`))
  (bind _temparray_2 (`local.TempArray`))
  (bind (_id _agent _kromosom _score) (break `/Game/Blueprints/Characters/BT/S_Kromosom` (`local.tempA`)))
  (bind (_id_2 _agent_2 _kromosom_2 _score_2) (break `/Game/Blueprints/Characters/BT/S_Kromosom` (`local.tempB`)))
  (`KismetArrayLibrary.Array_Clear` _temparray)
  (`KismetArrayLibrary.Array_Append` _temparray (`/Game/Blueprints/GI_Main.Get Top Chromosome` (`self.GetGI`) TargetArray 10))
  (bind _output_get (set `local.tempA` (`KismetArrayLibrary.Array_Random` _temparray_2)))
  (if (`self.isDoCrossover`)
    (`KismetArrayLibrary.Array_RemoveItem` _temparray_2 _output_get)
    (set `local.tempB` (`KismetArrayLibrary.Array_Random` _temparray_2))
    (bind _result (`/Game/Blueprints/GI_Main.Crossover & Mutation` (`self.GetGI`) (`local.tempA`) (`local.tempB`) (+ _id _id_2) (/ (+ _score _score_2) 2.0)))
    (return _result)
    (else
      (return (`local.tempA`)))))

(fn `Set New Pause`
  (params (`New Pause` :type Boolean))
  (bind _output_get (set `self.IsPause?` `New Pause`))
  (bind _returnvalue (`GameplayStatics.SetGamePaused` _output_get))
  (if (not _returnvalue)
    (`self.SetTimeDilation` (`self.SpeedMultiplier`)))
  (return))

(fn `SetTimeDilation`
  (params (TimeDilation :type "Float (single-precision)" :default 1.0))
  (`GameplayStatics.SetGlobalTimeDilation` TimeDilation)
  (return))

(fn `SpeedUp`
  (bind _output_get (set `self.SpeedMultiplier` (+ (`self.SpeedMultiplier`) (`self.SpeedMultiplierUp`))))
  (if (> _output_get (`self.MaxSpeedMultiplier`))
    (set `self.SpeedMultiplier` (`self.SpeedMultiplierUp`)))
  (`self.SetTimeDilation` (`self.SpeedMultiplier`))
  (return))

(fn `UserConstructionScript`)