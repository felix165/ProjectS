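; HUD_Main is a HUD Blueprint that currently provides only cached access to the main game instance and game mode.
; GetGI and GetGM return the stored reference, first casting to GI_Main or GM_Main and storing the result whenever the cached one is invalid.
; The event graph holds only disabled default events and the construction script is empty, so no drawing or widget logic is present.
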(fn `Get_GI`
  (returns (GI :type "/Game/Blueprints/GI_Main Object Reference"))
  (`self.GI`
    (:`then`
      _)
    (:`else`
      (bind _asgi_main (cast `/Game/Blueprints/GI_Main` (`GameplayStatics.GetGameInstance`))
        (:`then`
          (set `self.GI` _asgi_main))
        (:`CastFailed`
          _))))
  (return (`self.GI`)))

(fn `Get_GM`
  (returns (GM :type "/Game/Blueprints/GM_Main Object Reference"))
  (`self.GM`
    (:`then`
      _)
    (:`else`
      (bind _asgm_main (cast `/Game/Blueprints/GM_Main` (`GameplayStatics.GetGameMode`))
        (:`then`
          (set `self.GM` _asgm_main))
        (:`CastFailed`
          _))))
  (return (`self.GM`)))

(fn `UserConstructionScript`)