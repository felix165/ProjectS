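; Training manager that evolves chromosomes for AI agent teams through repeated battles in a grid of spawned arenas, with audio muted.
; Each iteration pairs shuffled team IDs, skipping blacklisted pairs, and arenas report results through FightFinished.
; Wins go to the GameInstance to update chromosomes; ties regenerate newly created ones or blacklist the pair.
; All-new populations retrain without counting the iteration; checkpoints save at milestones, ending at an iteration cap or exhausted pairings.
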(event `self.Init`
  (bind _gi_main (`self.GetGI`))
  (set `/Game/Blueprints/GI_Main.CurTrainingIteration` 0 _gi_main :!label _label)
  (set `/Game/Blueprints/GI_Main.TieCounter` 0 _gi_main)
  (`/Game/Blueprints/GI_Main.Generate First Generation_Cluster` _gi_main (`self.ClassAgent`) 32)
  (`self.Save Training` 0 true)
  (`GameplayStatics.SetSoundMixClassOverride` "/Game/Sounds/MasterSoundMix.MasterSoundMix" "/Game/Sounds/SC_Master.SC_Master" 0.0)
  (`GameplayStatics.PushSoundMixModifier` "/Game/Sounds/MasterSoundMix.MasterSoundMix")
  (for _index (range 32)
    (`KismetArrayLibrary.Array_Add` (`self.TempShuffle`) _index)
    (`KismetArrayLibrary.Array_Add` (`self.Id_NewGenerated`) _index))
  (`self.Start Next Training`))

(event `self.ReceiveBeginPlay`
  (goto _label))

(event `self.Start Next Training`
  (if (< (`/Game/Blueprints/GI_Main.CurTrainingIteration` (`self.GetGI`)) (`self.MaxIterasi`))
    (`self.Spawn Arena` (`self.ClassAgent`) 4 4 6)
    (`self.Generate Battle List` (`/Game/Blueprints/GI_Main.TSwordsManKromosom` (`self.GetGI`)))
    (bind _keys (`BlueprintMapLibrary.Map_Keys` (`self.Arena_Cluster`)))
    (for _array_element _keys
      (`/Engine/EditorBlueprintResources/StandardMacros.IsValid` _array_element
        (:`Is Valid`
          (`/Game/Blueprints/Property/BP_Arena.Start Training` _array_element))))
    (bind _traininginfo_cluster (`/Game/Blueprints/HUD_Main.TrainingInfo_Cluster` (`self.GetHUD`))
      (:`then`
        (`/Game/Blueprints/ClusterTraining/UI/WB_TrainingInfo_Cluster.Update` _traininginfo_cluster))
      (:`else`))
    (else
      (`self.Training Finished`))))

(event `self.Training Finished`
  ;[1 1 1] Training Finished
  (`KismetSystemLibrary.PrintString` "Training Finished" false)
  (`self.Save Training` (`/Game/Blueprints/GI_Main.CurTrainingIteration` (`self.GetGI`)) true))

(event `self.Save Training`
  (params (Epoch :type Integer) (`SaveAll?` :type Boolean))
  (bind _gm (`/Game/Blueprints/GI_Main.Get_GM` (`self.GetGI`)))
  (bind _returnvalue (`KismetStringLibrary.Concat_StrStr` "TrainingResult_Cluster_Ver5_" (`KismetStringLibrary.Conv_IntToString` Epoch) "Epoch" (`self.Agent`)))
  (set `/Game/Blueprints/GM_Main.SlotName` _returnvalue _gm)
  (`/Game/Blueprints/GM_Main.Save_Training_Result` _gm "NewEnumerator0" `SaveAll?`)
  (`KismetSystemLibrary.Delay` 1.0)
  (`KismetSystemLibrary.PrintString` _returnvalue))

(fn `FightFinished`
  (params (Arena :type "/Game/Blueprints/Property/BP_Arena Object Reference") (State :type "/Game/Blueprints/Property/E_BattleState Enum" :default "NewEnumerator0"))
  (locals (Id_Pair :type "/Game/Blueprints/Property/S_IdPair Structure"))
  (bind _gi_main (`self.GetGI`))
  (bind _id_pair_id_a (break `/Game/Blueprints/Property/S_IdPair` (`local.Id_Pair`)))
  (bind (_id_pair_id_a_2 _id_pair_id_b) (break `/Game/Blueprints/Property/S_IdPair` (`local.Id_Pair`)))
  (bind (_id_pair_id_a_3 _id_pair_id_b_2) (break `/Game/Blueprints/Property/S_IdPair` (`local.Id_Pair`)))
  (bind (_id_pair_id_a_4 _id_pair_id_b_3) (break `/Game/Blueprints/Property/S_IdPair` (`local.Id_Pair`)))
  (bind (_id_pair_id_a_5 _id_pair_id_b_4) (break `/Game/Blueprints/Property/S_IdPair` (`local.Id_Pair`)))
  (bind (_id_pair_id_a_6 _id_pair_id_b_5) (break `/Game/Blueprints/Property/S_IdPair` (`local.Id_Pair`)))
  (bind _arena (`local.Arena`))
  (bind _returnvalue (`BlueprintMapLibrary.Map_Length` (`self.Arena_Cluster`)))
  (bind _curtrainingiteration (`/Game/Blueprints/GI_Main.CurTrainingIteration` (`self.GetGI`)))
  (set `local.Id_Pair` (`BlueprintMapLibrary.Map_Find` (`self.Arena_Cluster`) _arena))
  (switch `/Game/Blueprints/Property/E_BattleState` (`local.State`)
    (:`NewEnumerator0`
      (return))
    (:`NewEnumerator1`
      (return))
    (:`NewEnumerator2`
      (`self.Remove From New Generated` _id_pair_id_a_4)
      (`self.RemoveFromBlacklist` (make `/Game/Blueprints/Property/S_IdPair` _id_pair_id_a_4 _id_pair_id_b_3))
      (bind _returnvalue_2 (`/Game/Blueprints/GI_Main.Fight Win_Cluster` _gi_main (`local.Id_Pair`) (`self.ClassAgent`)))
      (`KismetArrayLibrary.Array_AddUnique` (`self.Id_NewGenerated`) _returnvalue_2))
    (:`NewEnumerator3`
      (`self.Remove From New Generated` _id_pair_id_a_2)
      (`self.RemoveFromBlacklist` (make `/Game/Blueprints/Property/S_IdPair` _id_pair_id_b _id_pair_id_a_2))
      (bind _returnvalue_3 (`/Game/Blueprints/GI_Main.Fight Win_Cluster` _gi_main (make `/Game/Blueprints/Property/S_IdPair` _id_pair_id_b_5 _id_pair_id_a_6) (`self.ClassAgent`)))
      (`KismetArrayLibrary.Array_AddUnique` (`self.Id_NewGenerated`) _returnvalue_3))
    (:`NewEnumerator4`
      (`/Engine/EditorBlueprintResources/StandardMacros.IncrementInt` (`/Game/Blueprints/GI_Main.TieCounter` (`self.GetGI`))
        (:`  `
          (if (`KismetMathLibrary.BooleanNOR` (`self.OnNewGenerated?` _id_pair_id_a_5) (`self.OnNewGenerated?` _id_pair_id_b_4))
            (`self.AddToBlacklist` (make `/Game/Blueprints/Property/S_IdPair` _id_pair_id_a_5 _id_pair_id_b_4))
            (else
              (if (`self.OnNewGenerated?` _id_pair_id_a)
                (`self.RemoveAllFromBlacklist` _id_pair_id_a)
                (`self.Re-Generate Chromosome` _id_pair_id_a))
              (if (`self.OnNewGenerated?` _id_pair_id_b_2)
                (`self.RemoveAllFromBlacklist` _id_pair_id_b_2)
                (`self.Re-Generate Chromosome` _id_pair_id_b_2))))))))
  (`/Game/Blueprints/Property/BP_Arena.On Battle End` _arena)
  (bind _result (`/Engine/EditorBlueprintResources/StandardMacros.IncrementInt` (`self.TempCountArena`))
    (:`  `
      (if (== _result _returnvalue)
        (set `self.TempCountArena` 0)
        (`self.Filter Array Chromosome` "NewEnumerator0")
        (if (>= (`KismetArrayLibrary.Array_Length` (`self.Id_NewGenerated`)) (* _returnvalue 2))
          (`KismetSystemLibrary.PrintString` "ReTrain - NOT COUNTED AS ITERATION" false)
          (`self.Re-Train`)
          (return)
          (else
            (`/Engine/EditorBlueprintResources/StandardMacros.IncrementInt` _curtrainingiteration
              (:`  `
                (if (== _curtrainingiteration 5)
                  (`self.Save Training` _curtrainingiteration true :!label _label)
                  (elif (== _curtrainingiteration 10)
                    (goto _label)
                    (elif (== _curtrainingiteration 20)
                      (goto _label)
                      (elif (== _curtrainingiteration 50)
                        (goto _label)
                        (elif (== _curtrainingiteration 100)
                          (goto _label)
                          (else
                            _))))))
                (`self.Start Next Training`)
                (return)))))))))

(fn `Filter Array Chromosome`
  (params (Index :type "/Game/Blueprints/Characters/E_AgentClass Enum" :default "NewEnumerator0"))
  (locals (`Temp Id` :type Integer))
  (bind _gi_main (`self.GetGI`))
  (bind _temp_id (`local.Temp Id`))
  (`/Game/Blueprints/GI_Main.Filter Array Chromosome` _gi_main (`/Game/Blueprints/GI_Main.TSwordsManKromosom` _gi_main))
  (`/Game/Blueprints/GI_Main.Filter Array Chromosome` _gi_main (`/Game/Blueprints/GI_Main.TShooterKromosom` _gi_main))
  (bind (_result_ _other_) (`/Game/Blueprints/GI_Main.Filter Array Chromosome` _gi_main (`/Game/Blueprints/GI_Main.TStaffFighterKromosom` _gi_main)))
  (for _array_element _other_
    (set `local.Temp Id` (`.Id_11_37E72B9C49D3D54F99EF61A75A7FFB8F` (break `/Game/Blueprints/Characters/BT/S_Kromosom` _array_element)))
    (`self.RemoveAllFromBlacklist` _temp_id)
    (`self.Remove From New Generated` _temp_id))
  (return))

(fn `Generate Battle List`
  (params (`Team List` :type "Array of /Game/Blueprints/Characters/BT/S_Kromosom Structure (by ref)"))
  (locals (LoopLimit :type Integer) (TempInt :type Integer) (Id_Pair :type "/Game/Blueprints/Property/S_IdPair Structure"))
  (bind _tempshuffle (`self.TempShuffle`))
  (bind _team_list (`local.Team List`))
  (bind _arena_cluster (`self.Arena_Cluster`))
  (bind _tempshuffle_2 (`self.TempShuffle`))
  (bind _returnvalue (/ (`KismetArrayLibrary.Array_Length` _tempshuffle) 2))
  (for _ (range (+ (`local.LoopLimit`) 1))
    (`KismetArrayLibrary.Array_Shuffle` _tempshuffle)
    (set `local.TempInt` _returnvalue)
    (for _index (range _returnvalue)
      (bind _output_get (set `local.Id_Pair` (make `/Game/Blueprints/Property/S_IdPair` (`.Id_11_37E72B9C49D3D54F99EF61A75A7FFB8F` (break `/Game/Blueprints/Characters/BT/S_Kromosom` (`|GetArrayItem` _team_list (`|GetArrayItem` _tempshuffle_2 _index)))) (`.Id_11_37E72B9C49D3D54F99EF61A75A7FFB8F` (break `/Game/Blueprints/Characters/BT/S_Kromosom` (`|GetArrayItem` _team_list (`|GetArrayItem` _tempshuffle_2 (+ _index (`local.TempInt`)))))))))
      (if (`self.OnBlacklist?` (make `/Game/Blueprints/Property/S_IdPair` (break `/Game/Blueprints/Property/S_IdPair` _output_get) (`.Id_B_4_854B48FD466EDFF75A3918AC00925654` (break `/Game/Blueprints/Property/S_IdPair` _output_get))))
        ;[1 1 1] Re-Generate
        (`/Engine/EditorBlueprintResources/StandardMacros.IncrementInt` (`local.LoopLimit`)
          (:`  `
            (break)))
        (else
          (bind _keys (`BlueprintMapLibrary.Map_Keys` _arena_cluster))
          (`BlueprintMapLibrary.Map_Add` _arena_cluster (`|GetArrayItem` _keys _index) (`local.Id_Pair`)))))
    (if (== (`local.LoopLimit`) 1000)
      (`self.Training Finished`)
      (`KismetSystemLibrary.PrintString` "Training Finished, Caused by blacklist full" false)
      (set `self.MaxIterasi` (`/Game/Blueprints/GI_Main.CurTrainingIteration` (`self.GetGI`)))))
  (return))

(fn `Re-Generate Chromosome`
  (params (Id :type Integer))
  (locals (Class :type "/Game/Blueprints/Characters/E_AgentClass Enum"))
  (bind _gi_main (`self.GetGI`))
  (bind _gi_main_2 (`self.GetGI`))
  (bind _class (`local.Class`))
  (bind _maxcurid (`/Game/Blueprints/GI_Main.MaxCurId` _gi_main))
  (`KismetArrayLibrary.Array_RemoveItem` (`self.Id_NewGenerated`) Id)
  (for _array_element (`self.ClassAgent`)
    (set `local.Class` _array_element)
    (bind _result (`/Game/Blueprints/GI_Main.Generate New Kromosom` _gi_main _maxcurid (`local.Class`)))
    (`|VariableSetRef` (`|GetArrayItem` (select `/Game/Blueprints/Characters/E_AgentClass` _class :`NewEnumerator0` (`/Game/Blueprints/GI_Main.TSwordsManKromosom` _gi_main_2) :`NewEnumerator1` (`/Game/Blueprints/GI_Main.TShooterKromosom` _gi_main_2) :`NewEnumerator2` (`/Game/Blueprints/GI_Main.TStaffFighterKromosom` _gi_main_2)) (`/Game/Blueprints/GI_Main.Get Kromosom Index` _gi_main_2 (`local.Id`) _class)) _result))
  (`KismetArrayLibrary.Array_AddUnique` (`self.Id_NewGenerated`) _maxcurid)
  (`/Engine/EditorBlueprintResources/StandardMacros.IncrementInt` _maxcurid
    (:`  `
      (return))))

(fn `Spawn Arena`
  (params (`Agent Class_` :type "Array of /Game/Blueprints/Characters/E_AgentClass Enum (by ref)" :default _) (`Amount X` :type Integer) (`Amount Y` :type Integer) (TeamSize :type Integer))
  (`BlueprintMapLibrary.Map_Clear` (`self.Arena_Cluster`))
  (for _index (range (* `Amount X` `Amount Y`))
    (bind _returnvalue (`|SpawnActorFromClass` "/Game/Blueprints/ClusterTraining/BP_Arena_Cluster_1.BP_Arena_Cluster_1_C" (`KismetMathLibrary.MakeTransform` (`KismetMathLibrary.MakeVector` (* (mod _index (`local.Amount X`)) 10000) (* (/ _index (`local.Amount Y`)) 10000))) "Undefined" "OverrideRootScale" null self _index TeamSize (`local.Agent Class_`) true null))
    (`BlueprintMapLibrary.Map_Add` (`self.Arena_Cluster`) _returnvalue))
  (return))

(fn `UserConstructionScript`
  (`parent.UserConstructionScript`))