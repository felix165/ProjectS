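; Training game mode that seeds battle teams A and B with evolved swordsman, shooter and staff fighter chromosomes.
; It async-loads saved training results into the game instance, or creates an empty save if none exists.
; After loading, each team takes one random index across all three unit types, or optionally crossover-mutates two distinct random parents.
; Each training update marks all arena agents active before calling the parent logic.
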(event `self.Update Training Data`
  (params (`Is A win?` :type Boolean))
  (bind _arena (`/Game/Blueprints/GI_Main.GetBattleArena` (`self.GetGI`)))
  (bind _isagenta_active_ (`/Game/Blueprints/Property/BP_Arena.isAgentA_Active?` _arena))
  ;[1 0.7619 0] Update Training Every Play
  (bind _keys (`BlueprintMapLibrary.Map_Keys` _isagenta_active_))
  (for _array_element _keys
    (`BlueprintMapLibrary.Map_Add` _isagenta_active_ _array_element true)
    (`BlueprintMapLibrary.Map_Add` (`/Game/Blueprints/Property/BP_Arena.isAgentB_Active?` _arena) _array_element true))
  (`parent.Update Training Data` `Is A win?`))

(event `self.Load_Training_Result`
  (bind _gi_main (`self.GetGI`))
  (bind _slotname (`self.SlotName`))
  (bind _isdocrossover (`self.isDoCrossover`))
  ;[0 0.192 1] Saving_Event
  (bind _returnvalue (`GameplayStatics.DoesSaveGameExist` _slotname))
  (if _returnvalue
    (bind _savegame (`AsyncActionHandleSaveGame.AsyncLoadGameFromSlot` _slotname)
      (:`Completed`
        (bind _assg_training_result (cast `/Game/Blueprints/SG_TrainingResult` _savegame))
        (bind _output_get (set `self.SaveObject` _assg_training_result))
        (set `/Game/Blueprints/GI_Main.TSwordsManKromosom` (`/Game/Blueprints/SG_TrainingResult.TSwordsManKromosom` _output_get) _gi_main)
        (set `/Game/Blueprints/GI_Main.TShooterKromosom` (`/Game/Blueprints/SG_TrainingResult.TShooterKromosom` _output_get) _gi_main)
        (set `/Game/Blueprints/GI_Main.TStaffFighterKromosom` (`/Game/Blueprints/SG_TrainingResult.TStaffFighterKromosom` _output_get) _gi_main)
        (`self.RandomCluster_A` 0 31 _isdocrossover)
        (`self.RandomCluster_B` 0 31 _isdocrossover)
        (`KismetSystemLibrary.PrintString` "Load Finished")))
    (else
      (`KismetSystemLibrary.PrintString` "Save Slot doesnt exist" true true (struct :`G` 0.66 :`B` 1.0 :`A` 1.0) 2.0 "Save")
      (bind _returnvalue_2 (`GameplayStatics.CreateSaveGameObject` "/Game/Blueprints/SG_TrainingResult.SG_TrainingResult_C"))
      (`/Engine/EditorBlueprintResources/StandardMacros.IsValid` _returnvalue_2
        (:`Is Valid`
          (`AsyncActionHandleSaveGame.AsyncSaveGameToSlot` _returnvalue_2 (`self.SlotName`)
            (:`Completed`
              (`KismetSystemLibrary.PrintString` "create Save success"))))
        (:`Is Not Valid`
          (`KismetSystemLibrary.PrintString` "create save failed"))))))

(fn `RandomCluster_A`
  (params (Min :type Integer) (Max :type Integer) (IsDoCrossover :type Boolean))
  (locals (TempA :type Integer :default 0) (TempB :type Integer :default 0) (NewId :type Integer) (NewScore :type "Float (double-precision)") (TempChromosomeA :type "/Game/Blueprints/Characters/BT/S_Kromosom Structure") (TempChromosomeB :type "/Game/Blueprints/Characters/BT/S_Kromosom Structure"))
  (bind _returnvalue (`KismetMathLibrary.RandomIntegerInRange` Min Max))
  (bind _gi_main (`self.GetGI`))
  (bind _gi_main_2 (`self.GetGI`))
  (bind (_id _agent _kromosom _score) (break `/Game/Blueprints/Characters/BT/S_Kromosom` (`local.TempChromosomeA`)))
  (bind (_id_2 _agent_2 _kromosom_2 _score_2) (break `/Game/Blueprints/Characters/BT/S_Kromosom` (`local.TempChromosomeB`)))
  (bind _tswordsmankromosom (`/Game/Blueprints/GI_Main.TSwordsManKromosom` _gi_main_2))
  (bind _tshooterkromosom (`/Game/Blueprints/GI_Main.TShooterKromosom` _gi_main_2))
  (bind _tstafffighterkromosom (`/Game/Blueprints/GI_Main.TStaffFighterKromosom` _gi_main_2))
  (`KismetSystemLibrary.PrintString` "Team A - Cluster" false)
  (set `local.TempA` _returnvalue)
  (if IsDoCrossover
    ;[1 1 1] Re-Random
    (bind _output_get (set `local.TempB` _returnvalue :!label _label))
    (if (== _output_get (`local.TempA`))
      (goto _label)
      (else
        (set `local.TempChromosomeA` (`|GetArrayItem` _tswordsmankromosom (`local.TempA`)))
        (set `local.TempChromosomeB` (`|GetArrayItem` _tswordsmankromosom (`local.TempB`)))
        (set `local.NewId` (+ _id _id_2 10000))
        (set `local.NewScore` (+ (/ (+ _score _score_2) 10.0) 1.0))
        (bind _result (`/Game/Blueprints/GI_Main.Crossover & Mutation` _gi_main_2 (`local.TempChromosomeA`) (`local.TempChromosomeB`) (`local.NewId`) (`local.NewScore`)))
        (set `/Game/Blueprints/GI_Main.SwordsManKromosom_A` _result _gi_main_2)
        (set `local.TempChromosomeA` (`|GetArrayItem` _tshooterkromosom (`local.TempA`)))
        (set `local.TempChromosomeB` (`|GetArrayItem` _tshooterkromosom (`local.TempB`)))
        (bind _result_2 (`/Game/Blueprints/GI_Main.Crossover & Mutation` _gi_main_2 (`local.TempChromosomeA`) (`local.TempChromosomeB`) (`local.NewId`) (`local.NewScore`)))
        (set `/Game/Blueprints/GI_Main.ShooterKromosom_A` _result_2 _gi_main_2)
        (set `local.TempChromosomeA` (`|GetArrayItem` _tstafffighterkromosom (`local.TempA`)))
        (set `local.TempChromosomeB` (`|GetArrayItem` _tstafffighterkromosom (`local.TempB`)))
        (bind _result_3 (`/Game/Blueprints/GI_Main.Crossover & Mutation` _gi_main_2 (`local.TempChromosomeA`) (`local.TempChromosomeB`) (`local.NewId`) (`local.NewScore`)))
        (set `/Game/Blueprints/GI_Main.StaffFighterKromosom_A` _result_3 _gi_main_2)
        (return)))
    (else
      (set `/Game/Blueprints/GI_Main.SwordsManKromosom_A` (`|GetArrayItem` (`/Game/Blueprints/GI_Main.TSwordsManKromosom` _gi_main) (`local.TempA`)) _gi_main)
      (set `/Game/Blueprints/GI_Main.ShooterKromosom_A` (`|GetArrayItem` (`/Game/Blueprints/GI_Main.TShooterKromosom` _gi_main) (`local.TempA`)) _gi_main)
      (set `/Game/Blueprints/GI_Main.StaffFighterKromosom_A` (`|GetArrayItem` (`/Game/Blueprints/GI_Main.TStaffFighterKromosom` _gi_main) (`local.TempA`)) _gi_main)
      (return))))

(fn `RandomCluster_B`
  (params (Min :type Integer) (Max :type Integer) (IsDoCrossover :type Boolean))
  (locals (TempA :type Integer :default 0) (TempB :type Integer :default 0) (NewId :type Integer) (NewScore :type "Float (double-precision)") (TempChromosomeA :type "/Game/Blueprints/Characters/BT/S_Kromosom Structure") (TempChromosomeB :type "/Game/Blueprints/Characters/BT/S_Kromosom Structure"))
  (bind _returnvalue (`KismetMathLibrary.RandomIntegerInRange` Min Max))
  (bind _gi_main (`self.GetGI`))
  (bind _gi_main_2 (`self.GetGI`))
  (bind (_id _agent _kromosom _score) (break `/Game/Blueprints/Characters/BT/S_Kromosom` (`local.TempChromosomeA`)))
  (bind (_id_2 _agent_2 _kromosom_2 _score_2) (break `/Game/Blueprints/Characters/BT/S_Kromosom` (`local.TempChromosomeB`)))
  (bind _tswordsmankromosom (`/Game/Blueprints/GI_Main.TSwordsManKromosom` _gi_main_2))
  (bind _tshooterkromosom (`/Game/Blueprints/GI_Main.TShooterKromosom` _gi_main_2))
  (bind _tstafffighterkromosom (`/Game/Blueprints/GI_Main.TStaffFighterKromosom` _gi_main_2))
  (`KismetSystemLibrary.PrintString` "TeamB-Cluster")
  (set `local.TempA` _returnvalue)
  (if IsDoCrossover
    ;[1 1 1] Re-Random
    (bind _output_get (set `local.TempB` _returnvalue :!label _label))
    (if (== _output_get (`local.TempA`))
      (goto _label)
      (else
        (set `local.TempChromosomeA` (`|GetArrayItem` _tswordsmankromosom (`local.TempA`)))
        (set `local.TempChromosomeB` (`|GetArrayItem` _tswordsmankromosom (`local.TempB`)))
        (set `local.NewId` (+ _id _id_2 10000))
        (set `local.NewScore` (+ (/ (+ _score _score_2) 10.0) 1.0))
        (bind _result (`/Game/Blueprints/GI_Main.Crossover & Mutation` _gi_main_2 (`local.TempChromosomeA`) (`local.TempChromosomeB`) (`local.NewId`) (`local.NewScore`)))
        (set `/Game/Blueprints/GI_Main.SwordsManKromosom_B` _result _gi_main_2)
        (set `local.TempChromosomeA` (`|GetArrayItem` _tshooterkromosom (`local.TempA`)))
        (set `local.TempChromosomeB` (`|GetArrayItem` _tshooterkromosom (`local.TempB`)))
        (bind _result_2 (`/Game/Blueprints/GI_Main.Crossover & Mutation` _gi_main_2 (`local.TempChromosomeA`) (`local.TempChromosomeB`) (`local.NewId`) (`local.NewScore`)))
        (set `/Game/Blueprints/GI_Main.ShooterKromosom_B` _result_2 _gi_main_2)
        (set `local.TempChromosomeA` (`|GetArrayItem` _tstafffighterkromosom (`local.TempA`)))
        (set `local.TempChromosomeB` (`|GetArrayItem` _tstafffighterkromosom (`local.TempB`)))
        (bind _result_3 (`/Game/Blueprints/GI_Main.Crossover & Mutation` _gi_main_2 (`local.TempChromosomeA`) (`local.TempChromosomeB`) (`local.NewId`) (`local.NewScore`)))
        (set `/Game/Blueprints/GI_Main.StaffFighterKromosom_B` _result_3 _gi_main_2)
        (return)))
    (else
      (set `/Game/Blueprints/GI_Main.SwordsManKromosom_B` (`|GetArrayItem` (`/Game/Blueprints/GI_Main.TSwordsManKromosom` _gi_main) (`local.TempA`)) _gi_main)
      (set `/Game/Blueprints/GI_Main.ShooterKromosom_B` (`|GetArrayItem` (`/Game/Blueprints/GI_Main.TShooterKromosom` _gi_main) (`local.TempA`)) _gi_main)
      (set `/Game/Blueprints/GI_Main.StaffFighterKromosom_B` (`|GetArrayItem` (`/Game/Blueprints/GI_Main.TStaffFighterKromosom` _gi_main) (`local.TempA`)) _gi_main)
      (return))))

(fn `UserConstructionScript`
  (`parent.UserConstructionScript`))