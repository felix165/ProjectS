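; BP_Shooter is a ranged attacker character that fires a projectile when its attack state event fires with EndState set.
; StateAttack plays the shoot sound at AttackSoundOrigin, then spawns a BP_ShooterProjectile at ProjectileOrigin, ignoring collisions.
; The projectile receives the HitEmitter and the shooter as its Agent, then is launched immediately.
; BeginPlay, overlap, Tick and the construction script add no logic beyond the parent.
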(event `self.State Attack`
  (params (`EndState?` :type Boolean))
  (bind (_returnvalue_location _returnvalue_rotation) (`KismetMathLibrary.BreakTransform` (`SceneComponent.K2_GetComponentToWorld` (`self.ProjectileOrigin`))))
  (if `EndState?`
    (`GameplayStatics.PlaySoundAtLocation` (`self.ShootSFX`) (`SceneComponent.K2_GetComponentLocation` (`self.AttackSoundOrigin`)) (struct) 1.0 1.0 0.0 null null null null)
    (bind _returnvalue (`|SpawnActorFromClass` "/Game/Blueprints/Characters/Projectile/BP_ShooterProjectile.BP_ShooterProjectile_C" (`KismetMathLibrary.MakeTransform` _returnvalue_location _returnvalue_rotation) "AlwaysSpawn" "OverrideRootScale" null (`self.Hit Emitter`) 1.0 self null))
    (`/Game/Blueprints/Characters/Projectile/BP_ProjectileBase.Launch` _returnvalue true)))

(fn `UserConstructionScript`
  (`parent.UserConstructionScript`))