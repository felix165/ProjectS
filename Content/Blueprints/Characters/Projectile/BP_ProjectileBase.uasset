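; Base projectile actor that flies forward once launched and reports capsule hits to the Agent it references.
; A gate toggled by Launch lets Tick move it without sweep along the Projectile component's forward vector at scaled launch speed.
; Accepted hits and non-agent overlaps spawn an emitter at a line-traced impact point and destroy it; rejected agents are passed through.
; Without a valid Agent, any overlap just destroys it.
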(event `self.ReceiveTick`
  (params (DeltaSeconds :type "Float (single-precision)"))
  (`/Engine/EditorBlueprintResources/StandardMacros.Gate` true :!label _label
    (:`Exit`
      (`self.SetForward` DeltaSeconds))))

(event `Launch`
  (params (`isActive?` :type Boolean))
  (if `isActive?`
    (goto _label :!via `Open`)
    (else
      (goto _label :!via `Close`))))

(event `self.CapsuleCollider.OnComponentBeginOverlap`
  (params (OverlappedComponent :type "PrimitiveComponent Object Reference") (OtherActor :type "Actor Object Reference") (OtherComp :type "PrimitiveComponent Object Reference") (OtherBodyIndex :type Integer) (bFromSweep :type Boolean) (SweepResult :type "HitResult Structure (by ref)"))
  (bind _agent (`self.Agent`)
    (:`then`
      (bind _ishit_ (`/Game/Blueprints/Characters/BP_BaseAgent.WeaponBeginOverlap` _agent OverlappedComponent OtherActor OtherComp OtherBodyIndex bFromSweep SweepResult))
      (if (not _ishit_)
        (cast `/Game/Blueprints/Characters/BP_BaseAgent` OtherActor
          (:`CastFailed`
            _)))
      (bind _outhit (`KismetSystemLibrary.LineTraceSingleForObjects` (`self.K2_GetActorLocation`) (`self.K2_GetActorLocation` (`.HitActor` (`GameplayStatics.BreakHitResult` SweepResult))) (`|MakeArray` "ObjectTypeQuery7" :!type "EObjectTypeQuery Enum")))
      (`GameplayStatics.SpawnEmitterAtLocation` (`self.Hit Emitter`) (`.ImpactPoint` (`GameplayStatics.BreakHitResult` _outhit)) (struct) (2.0 2.0 2.0))
      (`self.K2_DestroyActor`))
    (:`else`
      (`self.K2_DestroyActor`))))

(fn `SendOverlapToOwner`
  (params (Actor :type "Object Object Reference")))

(fn `SetForward`
  (params (DeltaTime :type "Float (double-precision)"))
  (`self.K2_AddActorWorldOffset` (* (* DeltaTime (`SceneComponent.GetForwardVector` (`self.Projectile`))) (* (`self.LaunchSpeed`) (`self.LaunchSpeedMultiplier`))))
  (return))

(fn `UserConstructionScript`)